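; Character Blueprint that applies up to four decals to itself, one slot at a time, tracked by DecalSort.
; Set copies material and offset UI location from the dt_game_state game instance onto the current slot's decal component, raises its sort order and sets AniStatusIdle.
; Move reverts that slot to Mi_com_decal_000 while DecalSortMI marks it pending.
; SetDecalSort advances the slot and clears that flag if any decal differs from that material.
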(event Custom|Cus_Decal_MoveDecal
  (bind _decalsort (Variables|Default|GetDecalSort))
  (bind _decalsortmi (Variables|Default|GetDecalSortMI))
  ;[1 1 1] 设置贴花
  (Utilities|FlowControl|Sequence
    (:then_0
      (CallFunction|FunMoveDecal (Variables|Default|GetDecal_01) (and (== _decalsort 0) _decalsortmi)))
    (:then_1
      (CallFunction|FunMoveDecal (Variables|Default|GetDecal_02) (and (== _decalsort 1) _decalsortmi)))
    (:then_2
      (CallFunction|FunMoveDecal (Variables|Default|GetDecal_03) (and (== _decalsort 2) _decalsortmi)))
    (:then_3
      (CallFunction|FunMoveDecal (Variables|Default|GetDecal_04) (and (== _decalsort 3) _decalsortmi)))))

(event Custom|Cus_Decal_SetDecalSort
  ;[1 1 1] 设置贴花
  (if (or (or (!= (Variables|/Script/Engine.DecalComponent|GetDecalMaterial (Variables|Default|GetDecal_02)) "/Game/art/common/materials/mi_com_decal_000.mi_com_decal_000") (!= (Variables|/Script/Engine.DecalComponent|GetDecalMaterial (Variables|Default|GetDecal_01)) "/Game/art/common/materials/mi_com_decal_000.mi_com_decal_000")) (or (!= (Variables|/Script/Engine.DecalComponent|GetDecalMaterial (Variables|Default|GetDecal_03)) "/Game/art/common/materials/mi_com_decal_000.mi_com_decal_000") (!= (Variables|/Script/Engine.DecalComponent|GetDecalMaterial (Variables|Default|GetDecal_04)) "/Game/art/common/materials/mi_com_decal_000.mi_com_decal_000")))
    (Variables|Default|SetDecalSort (+ (Variables|Default|GetDecalSort) 1))
    (Variables|Default|SetDecalSortMI false)))

(event Custom|Cus_Decal_SetDecal
  (bind _decalsort (Variables|Default|GetDecalSort))
  ;[1 1 1] 设置贴花
  (if (== (Math|Integer|%(Integer) _decalsort 2) 0)
    (CallFunction|FunSetDecal (== _decalsort 0) (Variables|Default|GetDecal_01))
    (CallFunction|FunSetDecal (== _decalsort 2) (Variables|Default|GetDecal_03))
    (else
      (CallFunction|FunSetDecal (== _decalsort 1) (Variables|Default|GetDecal_02))
      (CallFunction|FunSetDecal (== _decalsort 3) (Variables|Default|GetDecal_04)))))

(event EventBeginPlay
  (bind _asdt_game_state (Utilities|Casting|CastTodt_game_state (Game|GetGameInstance)))
  (Variables|Default|SetDt%20Game%20State _asdt_game_state))

(event Collision|EventActorBeginOverlap
  (params (OtherActor :type Actor%20Object%20Reference)))

(event EventTick
  (params (DeltaSeconds :type Float%20%28single-precision%29)))

(fn ConstructionScript)

(fn FunSetDecal
  (params (Condition :type Boolean) (DecalLocation :type Decal%20Component%20Object%20Reference))
  (bind _dt_game_state (Variables|Default|GetDt%20Game%20State))
  (bind _tub_ui_decal_location (Variables|/Game/art/character/triple/triple_ur01_p_001/data/dt_game_state.dt_game_state_C|GetTub_UI_Decal_Location _dt_game_state))
  (if Condition
    (Rendering|Components|Decal|SetDecalMaterial DecalLocation (Variables|/Game/art/character/triple/triple_ur01_p_001/data/dt_game_state.dt_game_state_C|GetMI_Decal _dt_game_state))
    (Transformation|SetRelativeLocationAndRotation DecalLocation (Math|Vector|MakeVector (+ (.x _tub_ui_decal_location) 5e+01) (* (.y _tub_ui_decal_location) -1.0) (- (.z _tub_ui_decal_location) 8e+01)) "0.000000,0.000000,90.000000" false false)
    (Transformation|SetRelativeScale3D DecalLocation "0.100000,0.100000,0.100000")
    (Class|DecalComponent|SetSortOrder DecalLocation (+ (Variables|Default|GetDecalSort) 1))
    (Variables|/Game/art/character/triple/triple_ur01_p_001/data/dt_game_state.dt_game_state_C|SetAni_Status_Idle (Variables|Default|GetDt%20Game%20State) true)
    (Variables|Default|SetDecalSortMI true)))

(fn FunMoveDecal
  (params (Decal :type Decal%20Component%20Object%20Reference) (Condition :type Boolean))
  (if Condition
    (Rendering|Components|Decal|SetDecalMaterial Decal "/Game/art/common/materials/mi_com_decal_000.mi_com_decal_000")))