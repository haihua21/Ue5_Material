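; Character damage-decal Blueprint that sets up render-target painting on a skeletal mesh, apparently unfinished.
; BeginPlay clears the damage mask render target to black.
; UnWrap temporarily applies an unwrap material to slot 0, captures only that mesh with a rotated SceneCapture2D, then restores the original materials.
; Paint is a debug stub that only draws an arrow from the given position and normal and prints text.
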(event EventBeginPlay
  (Rendering|ClearRenderTarget2D "/Game/art/common/shaders/common/damage_decal/rt_crt_damage_mask.rt_crt_damage_mask"))

(fn ConstructionScript)

(fn UnWrap
  (bind _scenecapturecomponent2d (Variables|Default|GetSceneCaptureComponent2D))
  (bind _skeletalmesh (Variables|Default|GetSkeletalMesh))
  (Transformation|SetWorldRotation _scenecapturecomponent2d "-90.000000,-90.000000,0.000000" false false)
  (Rendering|SceneCapture|ShowOnlyComponent _scenecapturecomponent2d _skeletalmesh)
  (Variables|Default|SetTmp%20Materials (Rendering|Material|GetMaterials _skeletalmesh))
  (Rendering|Material|SetMaterial _skeletalmesh 0 "/Game/art/common/shaders/common/damage_decal/mat_unwrap.mat_unwrap")
  (Rendering|SceneCapture|CaptureScene (Variables|Default|GetSceneCaptureComponent2D) :!class /Script/Engine.SceneCaptureComponent2D)
  (for (_array_element _array_index) (Variables|Default|GetTmp%20Materials)
    (Rendering|Material|SetMaterial (Variables|Default|GetSkeletalMesh) _array_index _array_element)
    (Development|PrintText (Utilities|Text|ToText(Integer) _array_index))))

(fn Paint
  (params (Position :type Vector) (Normal :type Vector))
  (Rendering|Debug|DrawDebugArrow Position (* Normal 5e+01) 1.0 "(R=0.186344,G=0.378113,B=0.792708,A=1.000000)" 1.0 1.0)
  (Development|PrintText "print"))